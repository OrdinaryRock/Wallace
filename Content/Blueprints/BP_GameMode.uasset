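; Game mode that handles level progression, from level completion through to the game-complete screen.
; On BeginPlay it sets game-only input and looks up the current level name in the Levels array to cache the next entry, or "End" if none follows.
; LevelComplete shows a widget, then a timer calls LoadNextLevel to open that level or display the game-complete widget with UI-only input.
; EndGame opens Main1.
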(event `self.ReceiveBeginPlay`
  (bind _returnvalue (`GameplayStatics.GetPlayerController` 0))
  (bind _levels (`self.Levels`))
  (bind _returnvalue_2 (- (`KismetArrayLibrary.Array_Length` _levels) 1))
  (set `PlayerController.bShowMouseCursor` false _returnvalue)
  (`WidgetBlueprintLibrary.SetInputMode_GameOnly` _returnvalue)
  (bind _returnvalue_3 (`GameplayStatics.GetCurrentLevelName` true))
  (for (_array_element _array_index) _levels :!label _label
    (set `self.CurrentIndex` _array_index)
    (if (and (`KismetStringLibrary.EqualEqual_StrStr` _array_element _returnvalue_3) (< (`self.CurrentIndex`) _returnvalue_2))
      (set `self.NextLevel` (`|GetArrayItem` (`self.Levels`) (+ (`self.CurrentIndex`) 1)))
      (`self.BreakLoop`)
      (elif (== _returnvalue_2 (`self.CurrentIndex`))
        (set `self.NextLevel` "End")
        (`self.BreakLoop`)))))

(event `BreakLoop`
  (goto _label :!via `Break`))

(fn `EndGame`
  (`GameplayStatics.OpenLevel` "Main1"))

(fn `LevelComplete`
  (bind _returnvalue (`|CreateWidget` "/Game/Blueprints/WBP_LevelComplete.WBP_LevelComplete_C"))
  (bind _output_get (set `self.WBP_LevelComplete` _returnvalue))
  (`UserWidget.AddToViewport` _output_get 0)
  (`KismetSystemLibrary.K2_SetTimer` null "LoadNextLevel" 2.0))

(fn `LoadNextLevel`
  (bind _returnvalue (`GameplayStatics.GetPlayerController` 0))
  (bind _wbp_levelcomplete (`self.WBP_LevelComplete`))
  (if (`KismetStringLibrary.EqualEqual_StrStr` (`self.NextLevel`) "End")
    (`/Engine/EditorBlueprintResources/StandardMacros.IsValid` _wbp_levelcomplete
      (:`Is Valid`
        (`Widget.RemoveFromParent` _wbp_levelcomplete))
      (:`Is Not Valid`
        _))
    (bind _returnvalue_2 (`|CreateWidget` "/Game/Blueprints/WBP_GameComplete.WBP_GameComplete_C"))
    (`UserWidget.AddToViewport` _returnvalue_2 0)
    (set `PlayerController.bShowMouseCursor` true _returnvalue)
    (`WidgetBlueprintLibrary.SetInputMode_UIOnlyEx` _returnvalue _returnvalue_2)
    (else
      (`GameplayStatics.OpenLevel` (`KismetStringLibrary.Conv_StringToName` (`self.NextLevel`))))))

(fn `UserConstructionScript`)