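; BP_Player is the player of an obstacle-avoidance game, a physics-driven body pushed constantly forward and steered sideways.
; Tick adds a forward impulse and the MoveRight axis a lateral one, both scaled by mass and frame time.
; The lateral impulse is also applied as a velocity change.
; Hitting a BP_Obstacle calls GameEnded, which sets a flag that halts both impulses and prints a game-over message once.
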(event `self.ReceiveBeginPlay`)

(event `self.ReceiveTick`
  (params (DeltaSeconds :type "Float (single-precision)"))
  (bind _output_get (set `self.Delta Seconds` DeltaSeconds))
  (if (not (`self.bGameEnded`))
    (`PrimitiveComponent.AddImpulse` (`self.Player`) (`KismetMathLibrary.MakeVector` (* _output_get (* (`PrimitiveComponent.GetMass` (`self.Player`)) (`self.ForwardForce`))) 0.0 0.0) "None" false)))

(event `InputAxis|MoveRight`
  (params (AxisValue :type "Float (single-precision)"))
  (if (not (`self.bGameEnded`))
    (`PrimitiveComponent.AddImpulse` (`self.Player`) (`KismetMathLibrary.MakeVector` 0.0 (* AxisValue (* (`self.Delta Seconds`) (* (`self.SideForce`) (`PrimitiveComponent.GetMass` (`self.Player`)))))) "None" true)))

(event `self.Player.OnComponentHit`
  (params (HitComponent :type "PrimitiveComponent Object Reference") (OtherActor :type "Actor Object Reference") (OtherComp :type "PrimitiveComponent Object Reference") (NormalImpulse :type "Vector Structure") (Hit :type "HitResult Structure (by ref)"))
  (cast `/Game/Blueprints/BP_Obstacle` OtherActor)
  (`self.GameEnded`))

(fn `GameEnded`
  (if (not (`self.bGameEnded`))
    (set `self.bGameEnded` true)
    (`KismetSystemLibrary.PrintString` "Hit! Game over :(")))

(fn `UserConstructionScript`)